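; Player controller that owns the player's ammo count and handles the Fire and Reload inputs.
; Fire passes through AquireAmmo, which asks myGameState whether shooting is allowed and spends one round, then fires a bullet from the controlled myPawn and increments the game state's shot count.
; Reload refills ammo to the maximum, as on BeginPlay, and also calls RestartLevel on the game state.
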(event EventBeginPlay
  (CallFunction|Reload))

(event EventTick
  (params (DeltaSeconds :type Float%20%28single-precision%29)))

(event Input|ActionEvents|InputActionFire
  (params (Key :type Key%20Structure))
  (:Pressed
    (Utilities|AquireAmmo
      (:success
        (bind _asmy_pawn (Utilities|Casting|CastTomyPawn (Pawn|GetControlledPawn)))
        (Default|FireBullet _asmy_pawn)
        (bind _asmy_game_state (Utilities|Casting|CastTomyGameState (Game|GetGameState)))
        (Default|IncShotsMade _asmy_game_state)))))

(event Input|ActionEvents|InputActionReload
  (params (Key :type Key%20Structure))
  (:Pressed
    (CallFunction|TrytoRestart)
    (CallFunction|Reload)))

(fn ConstructionScript)

(fn Reload
  (Variables|Default|SetAmmo (Variables|Default|GetMaxAmmo)))

(fn TrytoRestart
  (bind _asmy_game_state (Utilities|Casting|CastTomyGameState (Game|GetGameState)))
  (Default|RestartLevel _asmy_game_state))