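; TargetMan is a shooting-target actor that pops on a rotating pivot and shatters when hit.
; After a random startup delay, a timeline drives the pivot's roll to show or hide the target.
; The first hit stops the timeline, swaps the intact body for pre-placed child pieces, and scatters them with physics and a radial impulse.
; It then increments the target-hit count on myGameState.
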(event Custom|ShowHideLoop
  (Utilities|FlowControl|Delay (Math|Random|RandomFloatinRange 0.0 5.0))
  (bind _rotation (Timeline|Timeline_0 Play)
    (:Update
      (Transformation|SetRelativeRotation (Variables|Default|GetRotationPivot) (Math|Rotator|MakeRotator (* _rotation 9e+01) 0.0 0.0) false false))))

(event EventBeginPlay
  (CallFunction|GetPartsArray)
  (CallFunction|SetPartsVisible false)
  (CallFunction|ShowHideLoop))

(event EventOnGetHit
  (if (Variables|Default|Getalive)
    (Variables|Default|Setalive false)
    (Utilities|FlowControl|Sequence
      (:then_0
        (bind _rotation (Timeline|Timeline_0 Stop)
          (:Update
            (Transformation|SetRelativeRotation (Variables|Default|GetRotationPivot) (Math|Rotator|MakeRotator (* _rotation 9e+01) 0.0 0.0) false false))))
      (:then_1
        (CallFunction|SetPartsVisible true)
        (CallFunction|SetPartsPhysicson)
        (CallFunction|MakeExplosion))
      (:then_2
        (bind _asmy_game_state (Utilities|Casting|CastTomyGameState (Game|GetGameState)))
        (Default|IncTargetHit _asmy_game_state)))))

(fn ConstructionScript)

(fn SetPartsVisible
  (params (new_visibility :type Boolean))
  ;[1 1 1] Parts visibility
  (Rendering|SetVisibility (Variables|Default|GetParts) new_visibility true)
  ;[1 1 1] Body visibility
  (Rendering|SetVisibility (Variables|Default|GetTargetBody) (not new_visibility) false))

(fn SetPartsPhysicson
  (for _array_element (Variables|Default|Getplate_parts)
    (bind _asstatic_mesh_component (Utilities|Casting|CastToStaticMeshComponent _array_element))
    (Physics|SetSimulatePhysics _asstatic_mesh_component true)))

(fn GetPartsArray
  (Variables|Default|Setplate_parts (Components|GetChildrenComponents (Variables|Default|GetParts) false)))

(fn MakeExplosion
  (for _array_element (Variables|Default|Getplate_parts)
    (bind _asstatic_mesh_component (Utilities|Casting|CastToStaticMeshComponent _array_element))
    (Physics|AddRadialImpulse _asstatic_mesh_component (Transformation|GetWorldLocation (Variables|Default|GetParts)) 5.0 2e+03 "RIF_Constant" false)))