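; Game state for a timed target-shooting level, tracking the round's phase, shots, hits and win or loss.
; On BeginPlay it counts TargetPlate and TargetMan actors as the goal, then runs a caption countdown before play starts.
; Tick shows the time left and declares a loss when time runs out; hitting all targets wins and reaching the ammo limit loses.
; CanShot permits firing only during play, and RestartLevel reloads the main level once the round ends.
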(event Custom|StartGame
  (Variables|Default|SetMainCaption "Get READY!")
  (Utilities|FlowControl|Delay 3.0)
  (Variables|Default|SetMainCaption "3")
  (Utilities|FlowControl|Delay 1.0)
  (Variables|Default|SetMainCaption "2")
  (Utilities|FlowControl|Delay 1.0)
  (Variables|Default|SetMainCaption "1")
  (Utilities|FlowControl|Delay 1.0)
  (Variables|Default|SetMainCaption "Go!")
  (Utilities|FlowControl|Delay 1.0)
  (CallFunction|StartCountDown))

(event Custom|StartCountDown
  (Variables|Default|Settemp_time (Utilities|Time|GetGameTimeinSeconds))
  (Variables|Default|Setgs "NewEnumerator1"))

(event EventBeginPlay
  (|SetTargetsCount
    (:out
      (CallFunction|StartGame))))

(event EventTick
  (params (DeltaSeconds :type Float%20%28single-precision%29))
  (bind (_secs _is_over) (CallFunction|GetRemaindSeconds))
  (switch Utilities|FlowControl|Switch|SwitchonEGameState (Variables|Default|Getgs)
    (:NewEnumerator1
      (if _is_over
        (Variables|Default|Setgs "NewEnumerator3")
        (Variables|Default|SetMainCaption "You loss!")
        (else
          (Variables|Default|SetMainCaption (Utilities|Text|ToText(String) (Utilities|String|Append "Time left: " (Utilities|String|ToString(Integer) (Math|Float|Floor _secs))))))))))

(fn ConstructionScript)

(fn GetRemaindSeconds
  (bind _returnvalue (Utilities|Time|GetGameTimeinSeconds))
  (bind _timelimit (Variables|Default|GetTimeLimit))
  (bind _temp_time (Variables|Default|Gettemp_time))
  (bind _returnvalue_2 (- _returnvalue _temp_time))
  (bind _returnvalue_3 (Math|Conversions|ToFloat(Integer) _timelimit))
  (bind _returnvalue_4 (- _returnvalue_3 _returnvalue_2))
  (return _returnvalue_4 (< _returnvalue_4 0.0)))

(fn IncTargetHit
  (bind _result (Math|Integer|IncrementInt (Variables|Default|GetTargetsHit))
    (:%20%20
      (if (>= _result (Variables|Default|GetTargetsCount))
        (Variables|Default|Setgs "NewEnumerator2")))))

(fn IncShotsMade
  (bind _result (Math|Integer|IncrementInt (Variables|Default|GetShotsMade))
    (:%20%20
      (if (>= _result (Variables|Default|GetAmmoLimit))
        (Variables|Default|Setgs "NewEnumerator3")))))

(fn CanShot
  (return (Utilities|Enum|Equal(Enum) (Variables|Default|Getgs) "NewEnumerator1")))

(fn RestartLevel
  (switch Utilities|FlowControl|Switch|SwitchonEGameState (Variables|Default|Getgs)
    (:NewEnumerator2
      _)
    (:NewEnumerator3
      _))
  (Game|OpenLevel(byName) "main"))