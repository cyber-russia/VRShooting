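; A player controller Blueprint that manages the player's ammo and handles the Fire and Reload inputs.
; Reload refills Ammo to MaxAmmo, both on BeginPlay and when Reload is pressed.
; Fire runs the AquireAmmo macro, which spends one round if any remain, and on success calls FireBullet on the controlled myPawn.
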(event EventBeginPlay
  (CallFunction|Reload))

(event EventTick
  (params (DeltaSeconds :type Float%20%28single-precision%29)))

(event Input|ActionEvents|InputActionFire
  (params (Key :type Key%20Structure))
  (:Pressed
    (Utilities|AquireAmmo
      (:success
        (bind _asmy_pawn (Utilities|Casting|CastTomyPawn (Pawn|GetControlledPawn)))
        (Default|FireBullet _asmy_pawn)))))

(event Input|ActionEvents|InputActionReload
  (params (Key :type Key%20Structure))
  (:Pressed
    (CallFunction|Reload)))

(fn ConstructionScript)

(fn Reload
  (Variables|Default|SetAmmo (Variables|Default|GetMaxAmmo)))